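; BP_QuestTriggerCollect is a quest trigger that advances a collection quest when tagged items enter its sphere.
; On sphere overlap it accepts actors carrying the configured ItemTag that are not yet in SeenItems, so each item counts once.
; Each new item is recorded, then the QuestManager on BP_MainGameMode receives CompleteQuest for the trigger's QuestId without completing the whole quest.
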(event `self.Sphere.OnComponentBeginOverlap`
  (params (OverlappedComponent :type "PrimitiveComponent Object Reference") (OtherActor :type "Actor Object Reference") (OtherComp :type "PrimitiveComponent Object Reference") (OtherBodyIndex :type Integer) (bFromSweep :type Boolean) (SweepResult :type "HitResult Structure (by ref)"))
  (if (and (`self.IsCorrectItem` OtherActor) (`self.HasNotSeenPumpkin` OtherActor))
    (`self.MarkItemSeen` OtherActor)
    (`self.NotifyQuestComplete`)))

(fn `HasNotSeenPumpkin`
  (params (ItemToFind :type "Actor Object Reference (by ref)"))
  (returns (ReturnValue :type Boolean))
  (return (not (`BlueprintSetLibrary.Set_Contains` (`self.SeenItems`) ItemToFind))))

(fn `IsCorrectItem`
  (params (self2 :type "Actor Object Reference"))
  (returns (ReturnValue :type Boolean))
  (return (`self.ActorHasTag` self2 (`self.ItemTag`))))

(fn `MarkItemSeen`
  (params (NewItem :type "Actor Object Reference (by ref)"))
  (`BlueprintSetLibrary.Set_Add` (`self.SeenItems`) NewItem))

(fn `NotifyQuestComplete`
  (bind _asbp_main_game_mode (cast `/Game/Core/BP_MainGameMode` (`GameplayStatics.GetGameMode`)))
  (`/Game/Quests/BP_QuestManager.CompleteQuest` (`/Game/Core/BP_MainGameMode.QuestManager` _asbp_main_game_mode) (`self.QuestId`) false))

(fn `UserConstructionScript`)