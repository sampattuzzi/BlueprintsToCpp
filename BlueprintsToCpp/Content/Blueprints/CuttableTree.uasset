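; Tree actor that falls over when hit by an actor tagged "Axe", completing the player's "Chop" quest.
; A mesh hit event passes through a DoOnce, stores the starting relative transform and plays the TreeFall timeline, which lerps the mesh toward TargetRotation.
; When the timeline finishes, it reports completion to the QuestManager on BP_MainGameMode.
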(event `self.Tree_Mesh.OnComponentHit`
  (params (HitComponent :type "PrimitiveComponent Object Reference") (OtherActor :type "Actor Object Reference") (OtherComp :type "PrimitiveComponent Object Reference") (NormalImpulse :type "Vector Structure") (Hit :type "HitResult Structure (by ref)"))
  (if (`self.ActorHasTag` OtherActor "Axe")
    (`/Engine/EditorBlueprintResources/StandardMacros.DoOnce` false
      (:`Completed`
        (set `self.StartRotation` (`SceneComponent.GetRelativeTransform` (`self.Tree_Mesh`)))
        (bind (_direction _rotation) (`Timeline|Tree Fall`)
          (:`Update`
            (`SceneComponent.K2_SetRelativeTransform` (`self.Tree_Mesh`) (`KismetMathLibrary.TLerp` (`self.StartRotation`) (`self.TargetRotation`) _rotation) false false))
          (:`Finished`
            (bind _asbp_main_game_mode (cast `/Game/Blueprints/BP_MainGameMode` (`GameplayStatics.GetGameMode`)))
            (`/Game/Blueprints/QuestManager.CompleteQuest` (`/Game/Blueprints/BP_MainGameMode.QuestManager` _asbp_main_game_mode) "Chop")))))))

(fn `UserConstructionScript`
  (`parent.UserConstructionScript`))